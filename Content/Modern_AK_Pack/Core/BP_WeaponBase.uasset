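; Base weapon Blueprint for the AK assault rifle, exposing Shoot, Reload and ReloadFull events that play the matching weapon montages on its skeletal mesh.
; Shoot also plays a 2D fire sound and spawns a shell casing at the ejection socket as the montage starts.
; The casing mesh ignores the first player's character when moving, and the events contain no hit or ammo logic.
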(event EventReloadFull
  ;[0.02604 0.006366 0.003613 1 11] Reload Full
  (Animation|Montage|PlayMontage (Variables|Default|GetSK_AssaultRifle) "/Game/Modern_AK_Pack/Art/AK/Animations/AM_FP_WEP_AK_Reload_Full.AM_FP_WEP_AK_Reload_Full"))

(event EventReload
  ;[0.02604 0.006366 0.003613 1 11] Reload
  (Animation|Montage|PlayMontage (Variables|Default|GetSK_AssaultRifle) "/Game/Modern_AK_Pack/Art/AK/Animations/AM_FP_WEP_AK_Reload.AM_FP_WEP_AK_Reload"))

(event EventShoot
  ;[0.02604 0.006366 0.003613] Shoot
  (Animation|Montage|PlayMontage (Variables|Default|GetSK_AssaultRifle) "/Game/Modern_AK_Pack/Art/AK/Animations/AM_FP_WEP_AK_Fire.AM_FP_WEP_AK_Fire"
    (:then
      ;[0 0 0 1 11] spawns a casing
      (Audio|PlaySound2D "/Game/Modern_AK_Pack/Art/AK/SOUND/FIRE/Cue_AK_Fire.Cue_AK_Fire" 1.0 1.0 0.0 0 0)
      (bind _returnvalue (Game|SpawnActorfromClass "/Game/Modern_AK_Pack/Core/BP_Casing.BP_Casing_C" (Transformation|GetSocketTransform (Variables|Default|GetSK_AssaultRifle) "SOCKET_Ejection" "RTS_World") "AlwaysSpawn" "MultiplyWithRoot" 0 0))
      (Collision|IgnoreActorwhenMoving (Variables|/Game/Modern_AK_Pack/Core/BP_Casing.BP_Casing_C|GetCasingMesh _returnvalue) (Game|GetPlayerCharacter 0) true))))

(fn ConstructionScript)